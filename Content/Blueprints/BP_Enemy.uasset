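; BP_Enemy is an enemy Blueprint that shows its health on a world-space widget bar.
; On BeginPlay it casts the EnemyHealth component's widget to BP_Enemy_health and caches the reference.
; Every Tick it sets the progress bar from Health, assuming a maximum of 100, and rotates the widget component to face the player camera as a billboard.
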(event `self.ReceiveBeginPlay`
  (bind _asbp_enemy_health (cast `/Game/Blueprints/BP_Enemy_health` (`WidgetComponent.GetUserWidgetObject` (`self.Enemy Health`))))
  (set `self.Enemy Health UI REF` _asbp_enemy_health))

(event `self.ReceiveTick`
  (params (DeltaSeconds :type "Float (single-precision)"))
  (bind _enemy_health (`self.Enemy Health`))
  (`ProgressBar.SetPercent` (`/Game/Blueprints/BP_Enemy_health.HealthProgressBar` (`self.Enemy Health UI REF`)) (/ (`self.Health`) 100.0))
  (`SceneComponent.K2_SetWorldRotation` _enemy_health (`KismetMathLibrary.FindLookAtRotation` (`SceneComponent.K2_GetComponentLocation` _enemy_health) (`SceneComponent.K2_GetComponentLocation` (`PlayerCameraManager.TransformComponent` (`GameplayStatics.GetPlayerCameraManager` 0)))) false false))

(fn `UserConstructionScript`)